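; Player controller for the BP_LeoSlider pawn that manages Enhanced Input mapping contexts and creates the HUD.
; Mouse-look input is added on BeginPlay for the local controller, while the pawn's OnGroundedChange event swaps between grounded and airborne contexts.
; On possess, it creates WB_HUD and hands its speed counter widget to the pawn.
; Possessing any other pawn type raises a script error and disables the controller's tick.
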(event Custom|OnGroundedChange
  (params (newGrounded :type Boolean))
  ;[0.15 0.15 0.15 0.5] Change IMC
  (if newGrounded
    (CallFunction|ChangeMappingContext "/Game/Inputs/IMC_Grounded.IMC_Grounded" "/Game/Inputs/IMC_Airborne.IMC_Airborne")
    (else
      (CallFunction|ChangeMappingContext "/Game/Inputs/IMC_Airborne.IMC_Airborne" "/Game/Inputs/IMC_Grounded.IMC_Grounded"))))

(event EventPossess
  (params (PossessedPawn :type Pawn%20Object%20Reference))
  ;[0.15 0.15 0.15 0.5] On Possess
  (bind _asbp_leo_slider (Utilities|Casting|CastToBP_LeoSlider PossessedPawn)
    (:then
      (bind _output_get (Variables|Default|SetPossessedPawn _asbp_leo_slider))
      (EventDispatchers|BindEventtoOnGroundedChange _output_get (EventDispatchers|CreateEvent :!event Custom|OnGroundedChange))
      (bind _returnvalue (UserInterface|CreateWidget "/Game/UI/WB_HUD.WB_HUD_C" self))
      (bind _output_get_2 (Variables|Default|SetHUD _returnvalue))
      (UserInterface|Viewport|AddtoPlayerScreen _output_get_2)
      (Variables|/Game/Pawns/BP_LeoSlider.BP_LeoSlider_C|SetSpeedWidget (Variables|Default|GetPossessedPawn) (Variables|/Game/UI/WB_HUD.WB_HUD_C|GetWB_SpeedCounter _returnvalue)))
    (:CastFailed
      ;;[0.6146 0.02328 0 0.5] Error Scenario, stops the ticking of this BP.
      (Utilities|Debugging|RaiseScriptError "Controlled Pawn is not BP_LeoSlider ! 
Can't adapt IMCs, stopping this class from ticking to avoid spamming...")
      (Actor|Tick|SetActorTickEnabled self))))

(event EventBeginPlay
  ;[0.15 0.15 0.15 0.5] Begin Play
  (if (Pawn|IsLocalPlayerController)
    (Input|AddMappingContext (PlayerController|LocalPlayerSubsystems|GetEnhancedInputLocalPlayerSubsystem self) "/Game/Inputs/IMC_MouseLook.IMC_MouseLook" 0 "(bIgnoreAllPressedKeysUntilRelease=True,bForceImmediately=False,bNotifyUserSettings=False)")))

(fn ConstructionScript)

(fn ChangeMappingContext
  (params (contextToAdd :type Input%20Mapping%20Context%20Object%20Reference) (contextToDel :type Input%20Mapping%20Context%20Object%20Reference))
  (bind _self self)
  (bind _returnvalue (PlayerController|LocalPlayerSubsystems|GetEnhancedInputLocalPlayerSubsystem _self))
  (Utilities|FlowControl|Sequence
    (:then_0
      (Input|RemoveMappingContext _returnvalue contextToDel "(bIgnoreAllPressedKeysUntilRelease=True,bForceImmediately=False,bNotifyUserSettings=False)"))
    (:then_1
      (Input|AddMappingContext _returnvalue contextToAdd 0 "(bIgnoreAllPressedKeysUntilRelease=True,bForceImmediately=False,bNotifyUserSettings=False)"))))