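; BP_BaptSlider is a prototype pawn with a Cube that the player tilts through weight-shift input, which adds roll and yaw rotation.
; A box collider tracks overlapping "Ground"-tagged actors in a set, which backs IsGrounded and a per-frame debug print.
; Move runs a downward trace whose result is unused, and MultWeight only prints.
; Center-of-mass shifting exists but is disconnected.
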(event OnComponentBeginOverlap(BoxColl)
  (params (OverlappedComponent :type Primitive%20Component%20Object%20Reference) (OtherActor :type Actor%20Object%20Reference) (OtherComp :type Primitive%20Component%20Object%20Reference) (OtherBodyIndex :type Integer) (bFromSweep :type Boolean) (SweepResult :type Hit%20Result%20Structure%20%28by%20ref%29))
  ;[0.03844 0.15 0.1033 0.5] Ground Detection
  (if (Actor|ActorHasTag OtherActor "Ground")
    (Utilities|Set|Add (Variables|Var|GroundDetection|GetcurGroundActorTouched) OtherActor)))

(event OnComponentEndOverlap(BoxColl)
  (params (OverlappedComponent :type Primitive%20Component%20Object%20Reference) (OtherActor :type Actor%20Object%20Reference) (OtherComp :type Primitive%20Component%20Object%20Reference) (OtherBodyIndex :type Integer))
  ;[0.03844 0.15 0.1033 0.5] Ground Detection
  (Utilities|Set|Remove (Variables|Var|GroundDetection|GetcurGroundActorTouched) OtherActor))

(event Input|EnhancedActionEvents|EnhancedInputActionIA_Move
  (params (ActionValue :type Vector%202D%20Structure) (ElapsedSeconds :type Float%20%28double-precision%29) (TriggeredSeconds :type Float%20%28double-precision%29) (InputAction :type Input%20Action%20Object%20Reference :default "/Game/Inputs/Actions/IA_Move.IA_Move"))
  (bind _cube (Variables|Default|GetCube))
  (bind _returnvalue (Transformation|GetWorldLocation _cube))
  (Development|PrintString "MOVE :D" true false "(R=0.000000,G=0.660000,B=1.000000,A=1.000000)" (Utilities|Time|GetWorldDeltaSeconds) "curMoveAction")
  (bind _outhit (Collision|LineTraceByChannel _returnvalue (+ _returnvalue "0.000000,0.000000,-50.000000") "TraceTypeQuery1" false 0 "None")))

(event Input|EnhancedActionEvents|EnhancedInputActionIA_ShiftWeight
  (params (ActionValue :type Vector%202D%20Structure) (ElapsedSeconds :type Float%20%28double-precision%29) (TriggeredSeconds :type Float%20%28double-precision%29) (InputAction :type Input%20Action%20Object%20Reference :default "/Game/Inputs/Actions/IA_ShiftWeight.IA_ShiftWeight"))
  (:Triggered
    (Development|PrintString "ROTAT-E >:(" true false "(R=0.000000,G=0.660000,B=1.000000,A=1.000000)" 2.0 "curMoveAction")
    (Transformation|AddRelativeRotation (Variables|Default|GetCube) (Math|Rotator|MakeRotator (* (.x ActionValue) 8.0) 0.0 0.0) false false)
    (Transformation|AddRelativeRotation (Variables|Default|GetCube) (Math|Rotator|MakeRotator 0.0 0.0 (* (.y ActionValue) 8.0)) false false)))

(event Input|EnhancedActionEvents|EnhancedInputActionIA_MultWeight
  (params (ActionValue :type Float%20%28double-precision%29) (ElapsedSeconds :type Float%20%28double-precision%29) (TriggeredSeconds :type Float%20%28double-precision%29) (InputAction :type Input%20Action%20Object%20Reference :default "/Game/Inputs/Actions/IA_MultWeight.IA_MultWeight"))
  (bind _returnvalue (Utilities|Time|GetWorldDeltaSeconds))
  (Development|PrintString "MULTWEIGTH >:]" true false "(R=0.000000,G=0.660000,B=1.000000,A=1.000000)" _returnvalue "curAction")
  (Development|PrintString (Utilities|String|ToString(Float) ActionValue) true false "(R=0.000000,G=0.660000,B=1.000000,A=1.000000)" _returnvalue "curAction"))

(event EventTick
  (params (DeltaSeconds :type Float%20%28single-precision%29))
  ;[0.15 0.15 0.15 0.5] Shows Ground collisions this frame
  (Variables|Var|GroundDetection|SetTMP%20allTouchedGroundActors "") ; Quick reset before name collection
  (bind _valuepin (Utilities|Set|ForEachLoop(Set) (Variables|Var|GroundDetection|GetcurGroundActorTouched))
    (:then
      ;;[0.15 0.15 0.15 0.5] Collects every name and puts them in the same String
      (Variables|Var|GroundDetection|SetTMP%20allTouchedGroundActors (Utilities|String|Append (Variables|Var|GroundDetection|GetTMP%20allTouchedGroundActors) (Utilities|String|ToString(Name) (Class|Actor|GetAttachParentSocketName _valuepin)) ", ")))
    (:CompletedPin
      (Development|PrintString (Variables|Var|GroundDetection|GetTMP%20allTouchedGroundActors) true true "(R=0.331622,G=0.472882,B=1.000000,A=1.000000)" DeltaSeconds))))

(fn ConstructionScript)

(fn IsGrounded
  (return (> (Utilities|Set|Length (Variables|Var|GroundDetection|GetcurGroundActorTouched)) 0)))