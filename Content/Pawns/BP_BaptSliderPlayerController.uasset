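; Player controller for the BaptSlider pawn that swaps Enhanced Input mapping contexts based on whether the pawn is grounded or airborne.
; BeginPlay adds a persistent mouse-look context.
; Each tick checks the pawn's IsGrounded state, adding the grounded or airborne context if missing, removing the other and printing a debug message.
; If the pawn is not a BP_BaptSlider, it raises a script error and disables its own tick.
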(event EventTick
  (params (DeltaSeconds :type Float%20%28single-precision%29))
  (bind _self self)
  (bind _returnvalue (PlayerController|LocalPlayerSubsystems|GetEnhancedInputLocalPlayerSubsystem _self))
  (bind _asbp_bapt_slider (Utilities|Casting|CastToBP_BaptSlider (Game|Player|GetPlayerPawn 0))
    (:then
      (bind _res (Default|IsGrounded _asbp_bapt_slider))
      (if _res
        (bind _returnvalue_2 (Class|EnhancedInputSubsystemInterface|HasMappingContext(Message) _returnvalue "/Game/Inputs/IMC_Grounded.IMC_Grounded"))
        (if (not _returnvalue_2)
          (Input|AddMappingContext _returnvalue "/Game/Inputs/IMC_Grounded.IMC_Grounded" 0 "(bIgnoreAllPressedKeysUntilRelease=True,bForceImmediately=False,bNotifyUserSettings=False)")
          (Input|RemoveMappingContext _returnvalue "/Game/Inputs/IMC_Airborne.IMC_Airborne" "(bIgnoreAllPressedKeysUntilRelease=True,bForceImmediately=False,bNotifyUserSettings=False)")
          (Development|PrintString "Added Grounded controls !" true true "(R=1.000000,G=0.040915,B=0.000000,A=1.000000)" 2.0 "changedIMC"))
        (else
          (bind _returnvalue_3 (Class|EnhancedInputSubsystemInterface|HasMappingContext(Message) _returnvalue "/Game/Inputs/IMC_Airborne.IMC_Airborne"))
          (if (not _returnvalue_3)
            (Input|AddMappingContext _returnvalue "/Game/Inputs/IMC_Airborne.IMC_Airborne" 0 "(bIgnoreAllPressedKeysUntilRelease=True,bForceImmediately=False,bNotifyUserSettings=False)")
            (Input|RemoveMappingContext _returnvalue "/Game/Inputs/IMC_Grounded.IMC_Grounded" "(bIgnoreAllPressedKeysUntilRelease=True,bForceImmediately=False,bNotifyUserSettings=False)")
            (Development|PrintString "Added Airborne controls !" true true "(R=1.000000,G=0.040915,B=0.000000,A=1.000000)" 2.0 "changedIMC")))))
    (:CastFailed
      ;[0.6146 0.02328 0 0.5] Error Scenario, stops the ticking of this BP.
      (Utilities|Debugging|RaiseScriptError "Controlled Pawn is not BP_BaptSlider ! 
Can't adapt IMCs, stopping this class from ticking to avoid spamming...")
      (Actor|Tick|SetActorTickEnabled self))))

(event EventBeginPlay
  (Input|AddMappingContext (PlayerController|LocalPlayerSubsystems|GetEnhancedInputLocalPlayerSubsystem self) "/Game/Inputs/IMC_MouseLook.IMC_MouseLook" 0 "(bIgnoreAllPressedKeysUntilRelease=True,bForceImmediately=False,bNotifyUserSettings=False)"))

(fn ConstructionScript)