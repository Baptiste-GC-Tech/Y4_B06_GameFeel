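; BP_Particles is an actor that toggles a Niagara slide particle effect based on the movement of its Cube component.
; Each tick it feeds the Cube's negated forward vector to the NiagaraForward parameter and prints the forward vector for debugging.
; IsAirborne becomes true when X or Z velocity is exactly zero, deactivating the particles; otherwise they activate.
; BeginPlay uses the flag the opposite way, activating particles when it is true.
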(event Collision|EventActorBeginOverlap
  (params (OtherActor :type Actor%20Object%20Reference)))

(event EventTick
  (params (DeltaSeconds :type Float%20%28single-precision%29))
  (bind _cube (Variables|Default|GetCube))
  (bind _returnvalue (Transformation|GetComponentVelocity _cube))
  (bind _returnvalue_2 (Math|Vector|GetForwardVector _cube))
  (bind (_x _y _z) (Math|Vector|BreakVector _returnvalue))
  (Niagara|SetNiagaraVariable(Vector3) (Variables|Default|GetNS_SlideParticles) "NiagaraForward" (* _returnvalue_2 "-1.000000,-1.000000,-1.000000"))
  (Development|PrintString (Utilities|String|ToString(Vector) _returnvalue_2))
  (bind _output_get (Variables|Default|SetIsAirborne (or (== _x 0.0) (== _z 0.0))))
  (if _output_get
    (Components|Activation|Deactivate (Variables|Default|GetNS_SlideParticles))
    (else
      (Components|Activation|Activate (Variables|Default|GetNS_SlideParticles) false))))

(event EventBeginPlay
  (if (Variables|Default|GetIsAirborne)
    (Components|Activation|Activate (Variables|Default|GetNS_SlideParticles) false)
    (else
      (Components|Activation|Deactivate (Variables|Default|GetNS_SlideParticles)))))

(fn ConstructionScript)