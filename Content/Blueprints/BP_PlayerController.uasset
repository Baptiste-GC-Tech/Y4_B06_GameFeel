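; Player controller Blueprint that switches Enhanced Input mapping contexts between ground and airborne controls.
; On BeginPlay, a local controller adds the grounded and mouse-look contexts.
; Every Tick it checks whether player pawn 0's movement component is falling, then swaps IMC_Grounded and IMC_Airborne if the needed one is missing, printing a debug message on each swap.
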(event EventTick
  (params (DeltaSeconds :type Float%20%28single-precision%29))
  (bind _self self)
  (bind _returnvalue (PlayerController|LocalPlayerSubsystems|GetEnhancedInputLocalPlayerSubsystem _self))
  (bind _returnvalue_2 (PlayerController|LocalPlayerSubsystems|GetEnhancedInputLocalPlayerSubsystem _self))
  (if (AI|Components|NavMovement|IsFalling (Pawn|GetMovementComponent (Game|Player|GetPlayerPawn 0)))
    (bind _returnvalue_3 (Class|EnhancedInputSubsystemInterface|HasMappingContext(Message) _returnvalue "/Game/Inputs/IMC_Airborne.IMC_Airborne"))
    (if (not _returnvalue_3)
      (Input|AddMappingContext _returnvalue "/Game/Inputs/IMC_Airborne.IMC_Airborne" 0 "(bIgnoreAllPressedKeysUntilRelease=True,bForceImmediately=False,bNotifyUserSettings=False)")
      (Input|RemoveMappingContext _returnvalue "/Game/Inputs/IMC_Grounded.IMC_Grounded" "(bIgnoreAllPressedKeysUntilRelease=True,bForceImmediately=False,bNotifyUserSettings=False)")
      (Development|PrintString "Added Airborne controls !" true true "(R=1.000000,G=0.040915,B=0.000000,A=1.000000)"))
    (else
      (bind _returnvalue_4 (Class|EnhancedInputSubsystemInterface|HasMappingContext(Message) _returnvalue_2 "/Game/Inputs/IMC_Grounded.IMC_Grounded"))
      (if (not _returnvalue_4)
        (Input|AddMappingContext _returnvalue_2 "/Game/Inputs/IMC_Grounded.IMC_Grounded" 0 "(bIgnoreAllPressedKeysUntilRelease=True,bForceImmediately=False,bNotifyUserSettings=False)")
        (Input|RemoveMappingContext _returnvalue_2 "/Game/Inputs/IMC_Airborne.IMC_Airborne" "(bIgnoreAllPressedKeysUntilRelease=True,bForceImmediately=False,bNotifyUserSettings=False)")
        (Development|PrintString "Added Ground controls !" true true "(R=1.000000,G=0.040915,B=0.000000,A=1.000000)")))))

(event EventBeginPlay
  (bind _returnvalue (PlayerController|LocalPlayerSubsystems|GetEnhancedInputLocalPlayerSubsystem))
  (if (Pawn|IsLocalPlayerController)
    (Utilities|FlowControl|Sequence
      (:then_0
        (Input|AddMappingContext _returnvalue "/Game/Inputs/IMC_Grounded.IMC_Grounded" 0 "(bIgnoreAllPressedKeysUntilRelease=True,bForceImmediately=False,bNotifyUserSettings=False)"))
      (:then_1
        (Input|AddMappingContext _returnvalue "/Game/Inputs/IMC_MouseLook.IMC_MouseLook" 0 "(bIgnoreAllPressedKeysUntilRelease=True,bForceImmediately=False,bNotifyUserSettings=False)")))))

(fn ConstructionScript)