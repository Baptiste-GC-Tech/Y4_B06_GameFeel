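; Sound manager that plays hard body-impact sounds when the BP_LeoSlider pawn lands.
; On BeginPlay it finds the BP_LeoSlider actor, caches it as PossessedPawn and binds to its OnGroundedChange event.
; When the grounded state turns true, a random switch picks one of six impact variants and plays it at the pawn's location.
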(event Custom|PlayCollideSFX
  (params (newGrounded :type Boolean))
  (bind _possessedpawn (Variables|Default|GetPossessedPawn))
  (bind _returnvalue (Transformation|GetActorLocation _possessedpawn))
  (if newGrounded
    (switch int (Math|Random|RandomIntegerinRange 0 5)
      (:0
        (Audio|PlaySoundatLocation "/Game/Sounds/SFX/body_medium_impact_hard1.body_medium_impact_hard1" _returnvalue "0, 0, 0" 1.0 1.0 0.0 0 0 0 0))
      (:1
        (Audio|PlaySoundatLocation "/Game/Sounds/SFX/body_medium_impact_hard2.body_medium_impact_hard2" _returnvalue "0, 0, 0" 1.0 1.0 0.0 0 0 0 0))
      (:2
        (Audio|PlaySoundatLocation "/Game/Sounds/SFX/body_medium_impact_hard3.body_medium_impact_hard3" _returnvalue "0, 0, 0" 1.0 1.0 0.0 0 0 0 0))
      (:3
        (Audio|PlaySoundatLocation "/Game/Sounds/SFX/body_medium_impact_hard4.body_medium_impact_hard4" _returnvalue "0, 0, 0" 1.0 1.0 0.0 0 0 0 0))
      (:4
        (Audio|PlaySoundatLocation "/Game/Sounds/SFX/body_medium_impact_hard5.body_medium_impact_hard5" _returnvalue "0, 0, 0" 1.0 1.0 0.0 0 0 0 0))
      (:5
        (Audio|PlaySoundatLocation "/Game/Sounds/SFX/body_medium_impact_hard6.body_medium_impact_hard6" _returnvalue "0, 0, 0" 1.0 1.0 0.0 0 0 0 0)))))

(event EventBeginPlay
  (Utilities|FlowControl|Sequence
    (:then_0
      (bind _returnvalue (Actor|GetActorOfClass "/Game/Pawns/BP_LeoSlider.BP_LeoSlider_C"))
      (Variables|Default|SetPossessedPawn _returnvalue)
      (EventDispatchers|BindEventtoOnGroundedChange _returnvalue (delegate Custom|PlayCollideSFX)))))

(fn ConstructionScript)